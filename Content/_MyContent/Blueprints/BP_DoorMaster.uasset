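; Base double-door actor that opens and closes two door meshes with a timeline, toggled by player interaction or character overlap.
; A FlipFlop alternates playing and reversing the timeline and plays a sound, gated by IsLocked plus CanInteract or CanOverlap.
; Overlap toggles fire through a server-named event only when the first character enters the box or the last one leaves.
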(event Custom|Sound
  (Audio|PlaySoundatLocation (Variables|Settings|GetDoorSound) (Transformation|GetActorLocation) "0, 0, 0" 1.0 1.0 0.0 0 0 0 0))

(event Custom|Server_ToglleDoor
  (if (and (not (Variables|Settings|GetIsLocked)) (Variables|Settings|GetCanOverlap))
    (CallFunction|Sound)
    (Utilities|FlowControl|FlipFlop
      (:A
        (bind (_direction _doorleft _doorright) (Timeline|Timeline Play)
          (:Update
            (Transformation|SetRelativeLocation (Variables|Default|GetDoorL) _doorleft false false)
            (Transformation|SetRelativeLocation (Variables|Default|GetDoorR) _doorright false false))))
      (:B
        (Timeline|Timeline Reverse)))))

(event EventInteract
  (if (and (not (Variables|Settings|GetIsLocked)) (Variables|Settings|GetCanInteract))
    (CallFunction|Sound)
    (Utilities|FlowControl|FlipFlop
      (:A
        (bind (_direction _doorleft _doorright) (Timeline|Timeline Play)
          (:Update
            (Transformation|SetRelativeLocation (Variables|Default|GetDoorL) _doorleft false false)
            (Transformation|SetRelativeLocation (Variables|Default|GetDoorR) _doorright false false))))
      (:B
        (Timeline|Timeline Reverse)))))

(event Collision|EventActorBeginOverlap
  (params (OtherActor :type Actor%20Object%20Reference))
  (CallFunction|ToggleOverlapDoor OtherActor true)
  (if (Variables|Settings|GetCanInteract)
    (Utilities|Casting|CastToBP_Demo_Character OtherActor)))

(event Collision|EventActorEndOverlap
  (params (OtherActor :type Actor%20Object%20Reference))
  (CallFunction|ToggleOverlapDoor OtherActor false))

(fn ConstructionScript)

(fn ToggleOverlapDoor
  (params (Player :type Object%20Object%20Reference) (On :type Boolean))
  (bind _box (Variables|Default|GetBox))
  (bind _overlappingactors (Collision|GetOverlappingActors _box "/Script/Engine.Character" :!class /Script/Engine.PrimitiveComponent))
  (bind _returnvalue (Utilities|Array|Length _overlappingactors))
  (Utilities|Casting|CastToCharacter Player)
  (if (select On (not (> _returnvalue 1)) (not (>= _returnvalue 1)))
    (CallFunction|ServerToglleDoor)))